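; BPC_HealthSystem is an actor component that tracks health for BP_ThirdPersonCharacter and mirrors it on the HUD health bar.
; On BeginPlay it waits a tick, caches the owning character and initializes the bar as current over max health.
; DecreaseHealth subtracts damage unless already depleted and returns whether health is at or below zero, without clamping to zero.
; IncreaseHealth adds health capped at the maximum, and both functions refresh the bar.
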(event EventBeginPlay
  (Utilities|FlowControl|DelayUntilNextTick)
  (bind _asbp_third_person_character (Utilities|Casting|CastToBP_ThirdPersonCharacter (Components|GetOwner)))
  (Variables|Default|SetPlayer _asbp_third_person_character)
  (Progress|SetPercent (Variables|/Game/UI/WB_PlayerStatsHUD.WB_PlayerStatsHUD_C|GetHealthBar (Variables|/Game/ThirdPerson/Blueprints/BP_ThirdPersonCharacter.BP_ThirdPersonCharacter_C|GetHUD%20Widget (Variables|Default|GetPlayer))) (/ (Variables|Default|GetCurrentHealth) (Variables|Default|GetMax%20Health))))

(fn DecreaseHealth
  (params (Damage :type Float%20%28double-precision%29))
  (if (not (<= (Variables|Default|GetCurrentHealth) 0.0))
    (bind _output_get (Variables|Default|SetCurrentHealth (- (Variables|Default|GetCurrentHealth) Damage)))
    (Progress|SetPercent (Variables|/Game/UI/WB_PlayerStatsHUD.WB_PlayerStatsHUD_C|GetHealthBar (Variables|/Game/ThirdPerson/Blueprints/BP_ThirdPersonCharacter.BP_ThirdPersonCharacter_C|GetHUD%20Widget (Variables|Default|GetPlayer))) (/ _output_get (Variables|Default|GetMax%20Health)))
    (if (<= (Variables|Default|GetCurrentHealth) 0.0)
      _
      (else
        (return false))))
  (return true))

(fn IncreaseHealth
  (params (HealthGained :type Float%20%28double-precision%29))
  (Variables|Default|SetCurrentHealth (+ HealthGained (Variables|Default|GetCurrentHealth)))
  (if (> (Variables|Default|GetCurrentHealth) (Variables|Default|GetMax%20Health))
    (Variables|Default|SetCurrentHealth (Variables|Default|GetMax%20Health)))
  (Progress|SetPercent (Variables|/Game/UI/WB_PlayerStatsHUD.WB_PlayerStatsHUD_C|GetHealthBar (Variables|/Game/ThirdPerson/Blueprints/BP_ThirdPersonCharacter.BP_ThirdPersonCharacter_C|GetHUD%20Widget (Variables|Default|GetPlayer))) (/ (Variables|Default|GetCurrentHealth) (Variables|Default|GetMax%20Health))))