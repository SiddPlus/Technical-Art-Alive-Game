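; BP_Spikes is a spike hazard that damages and knocks back the third-person character while it overlaps the box.
; Begin overlap casts the other actor's instigator, sets a colliding flag, applies damage and launches player 0's character opposite the spikes' forward vector.
; A one-second Delay loops the damage and launch until end overlap clears the flag.
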(event OnComponentBeginOverlap(Box)
  (params (OverlappedComponent :type Primitive%20Component%20Object%20Reference) (OtherActor :type Actor%20Object%20Reference) (OtherComp :type Primitive%20Component%20Object%20Reference) (OtherBodyIndex :type Integer) (bFromSweep :type Boolean) (SweepResult :type Hit%20Result%20Structure%20%28by%20ref%29))
  (bind _asbp_third_person_character (Utilities|Casting|CastToBP_ThirdPersonCharacter (Game|GetInstigator OtherActor)))
  (Variables|Default|SetIsColliding true)
  (Game|Damage|ApplyDamage _asbp_third_person_character 4.0 0 0 :!label _label)
  (Character|LaunchCharacter (Game|GetPlayerCharacter 0) (* (Math|Vector|GetForwardVector (Transformation|GetActorRotation)) -3e+03) false false)
  (Utilities|FlowControl|Delay 1.0)
  (if (Variables|Default|GetIsColliding)
    (goto _label)))

(event OnComponentEndOverlap(Box)
  (params (OverlappedComponent :type Primitive%20Component%20Object%20Reference) (OtherActor :type Actor%20Object%20Reference) (OtherComp :type Primitive%20Component%20Object%20Reference) (OtherBodyIndex :type Integer))
  (Utilities|Casting|CastToBP_ThirdPersonCharacter (Game|GetInstigator OtherActor))
  (Variables|Default|SetIsColliding false))

(fn ConstructionScript)