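; BP_Checkpoint is a checkpoint actor that records a respawn point when the player pawn overlaps its Sphere.
; An IsPlayer macro filters the overlap, printing a debug "Hello" for other actors.
; For the player, it plays a ping sound, stores the Scene component's world transform and a checkpoint flag in BP_GameInstance, then calls SetStaticMesh on two mesh components.
; Nothing prevents repeat triggering.
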(event OnComponentBeginOverlap(Sphere)
  (params (OverlappedComponent :type Primitive%20Component%20Object%20Reference) (OtherActor :type Actor%20Object%20Reference) (OtherComp :type Primitive%20Component%20Object%20Reference) (OtherBodyIndex :type Integer) (bFromSweep :type Boolean) (SweepResult :type Hit%20Result%20Structure%20%28by%20ref%29))
  (|IsPlayer? OtherActor
    (:else
      (Development|PrintString "Hello"))
    (:then
      (Utilities|FlowControl|Sequence
        (:then_0
          (|PlaySound))
        (:then_1
          (bind _asbp_game_instance (Utilities|Casting|CastToBP_GameInstance (Game|GetGameInstance)))
          (Variables|/Game/Blueprints/BP_GameInstance.BP_GameInstance_C|SetRespawnTransform _asbp_game_instance (Transformation|GetWorldTransform (Variables|Default|GetScene)))
          (Variables|/Game/Blueprints/BP_GameInstance.BP_GameInstance_C|SetCheckpointOn _asbp_game_instance true))
        (:then_2
          (|SetMeshes))))))

(event EventBeginPlay)

(event Collision|EventActorBeginOverlap
  (params (OtherActor :type Actor%20Object%20Reference)))

(event EventTick
  (params (DeltaSeconds :type Float%20%28single-precision%29)))

(fn ConstructionScript)