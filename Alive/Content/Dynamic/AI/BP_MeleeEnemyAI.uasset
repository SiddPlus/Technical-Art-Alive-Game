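; Melee enemy character that attacks the player with a two-swing sword combo and has its own health.
; Attack requests, apparently from a behavior tree, play montages by combo index, with SaveAttack gating continuation.
; A looping timer sphere-traces between two blade points while active, damaging the player with a brief cooldown.
; Taking damage triggers a grunt, hit montage and knockback, then ragdolls the enemy at zero health.
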(event Custom|Sword%20Attack%20Combo%20Call%20From%20BT
  ;[1 1 1] Combo System
  ;;[1 1 1] Attack
  (if (Variables|Default|GetCanAttack)
    (CallFunction|SwordAttack)))

(event Custom|Die
  (Input|DisableInput 0)
  (Physics|SetSimulatePhysics (Variables|Character|GetMesh) true))

(event Custom|Start%20Sword%20Trace
  ;[1 1 1] Sword Trace
  (bind _returnvalue (Utilities|Time|SetTimerbyEvent (delegate Custom|Sword%20Trace%20Loop) 0.001 true))
  (Variables|Default|SetSwordTraceLoop _returnvalue))

(event Custom|Sword%20Trace%20Loop
  (bind _returnvalue (Game|Player|GetPlayerPawn 0))
  ;[1 1 1] Sword Trace
  (bind _outhit (Collision|SphereTraceByChannel (Transformation|GetWorldLocation (Variables|Default|GetTopPoint)) (Transformation|GetWorldLocation (Variables|Default|GetBottomPoint)) 12.0 "TraceTypeQuery1" false 0 "ForDuration" true "(R=1.000000,G=0.000000,B=0.000000,A=1.000000)" "(R=0.000000,G=1.000000,B=0.000000,A=1.000000)" 0.2))
  (if (== (.HitActor (Collision|BreakHitResult _outhit)) _returnvalue)
    (Utilities|FlowControl|DoOnce false :!label _label
      (:Completed
        (Game|Damage|ApplyDamage _returnvalue 1.0 0 self)
        (CallFunction|PlaySound)
        (Utilities|FlowControl|Delay 0.5)
        (goto _label Reset)))))

(event Custom|Stop%20Sword%20Trace
  ;[1 1 1] Sword Trace
  (Utilities|Time|ClearandInvalidateTimerbyHandle (Variables|Default|GetSwordTraceLoop)))

(event Custom|Reaction
  (Audio|PlaySoundatLocation "/Game/Static/Audio/grunt-1-85280.grunt-1-85280" (Transformation|GetActorLocation) "0, 0, 0" 1.0 1.0 0.0 0 0 0 0)
  (Animation|PlayAnimMontage "/Game/Static/Animations/Reaction/Enemy_Hit_Reaction_Montage.Enemy_Hit_Reaction_Montage" 1.0 "None")
  (Character|LaunchCharacter (* (Math|Vector|GetForwardVector (Transformation|GetActorRotation)) -3e+02) false false))

(event Custom|Play%20Sound
  (Audio|PlaySoundatLocation "/Game/Static/Audio/hit-swing-sword-small-2-95566.hit-swing-sword-small-2-95566" (Transformation|GetActorLocation (Components|GetOwner)) "0, 0, 0" 1.0 1.0 0.0 0 0 0 0))

(event Custom|Sword%20Attack
  ;[1 1 1] Combo System
  ;;[1 1 1] Sword Attack
  (if (not (Variables|Default|GetIsAttacking))
    (Variables|Default|SetSaveAttack true)
    (switch int (Variables|Default|GetAttackIndex)
      (:0
        (|Attacks :!label _label))
      (:1
        (goto _label execute2)))))

(event Custom|Attack
  (params (AnimMontage :type Anim%20Montage%20Object%20Reference) (CurrentAttackIndex :type Integer))
  ;[1 1 1] Combo System
  ;;[1 1 1] Attack 1
  (Utilities|FlowControl|DoOnce false :!label _label
    (:Completed
      (Utilities|FlowControl|Delay 0.1)
      (Animation|Montage|PlayMontage (Variables|Character|GetMesh) AnimMontage (Variables|Default|GetSpeed)
        (:then
          (bind _result (Math|Integer|IncrementInt CurrentAttackIndex)
            (:%20%20
              (Variables|Default|SetAttackIndex _result)
              (goto _label Reset))))))))

(event Custom|Stop%20Combo
  ;[1 1 1] Combo System
  ;;[1 1 1] Stop Combo
  (Variables|Default|SetIsAttacking false)
  (Variables|Default|SetAttackIndex 0))

(event Custom|Sword%20Attack%20Combo
  ;[1 1 1] Combo System
  ;;[1 1 1] Continue Combo
  (if (Variables|Default|GetSaveAttack)
    (Variables|Default|SetSaveAttack false)
    (switch int (Variables|Default|GetAttackIndex)
      (:0
        (|Attacks :!label _label))
      (:1
        (goto _label execute2)))
    (else
      (CallFunction|StopCombo))))

(event Game|Damage|EventAnyDamage
  (params (Damage :type Float%20%28single-precision%29) (DamageType :type Damage%20Type%20Object%20Reference) (InstigatedBy :type Controller%20Object%20Reference) (DamageCauser :type Actor%20Object%20Reference))
  (bind _isenemydead (CallFunction|DecreaseHealth Damage))
  (CallFunction|Reaction)
  (if _isenemydead
    (CallFunction|Die)))

(event EventBeginPlay
  (Variables|Default|SetCurrentHealth (Variables|Default|GetMaxHealth)))

(fn ConstructionScript)

(fn DecreaseHealth
  (params (Damage :type Float%20%28double-precision%29))
  (if (not (<= (Variables|Default|GetCurrentHealth) 0.0))
    (Variables|Default|SetCurrentHealth (- (Variables|Default|GetCurrentHealth) Damage))
    (if (<= (Variables|Default|GetCurrentHealth) 0.0)
      _
      (else
        (return false))))
  (return true))

(fn Attack
  (CallFunction|SwordAttackComboCallfromBT)
  (return 0.4))