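; BPC_CollectablesSystem is a component that tracks the third-person character's coin wallet and shows it on the HUD.
; On BeginPlay it waits one tick, casts its owner to BP_ThirdPersonCharacter, caches it and sets the initial coin text.
; AddCoins adds the given amount to the wallet and refreshes the formatted CoinsText in the player's HUD widget.
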(event EventBeginPlay
  (Utilities|FlowControl|DelayUntilNextTick)
  (bind _asbp_third_person_character (Utilities|Casting|CastToBP_ThirdPersonCharacter (Components|GetOwner)))
  (Variables|Default|SetPlayer _asbp_third_person_character)
  (Rendering|Components|TextRender|SetText (Variables|/Game/Dynamic/UI/WB_PlayerStatsHUD.WB_PlayerStatsHUD_C|GetCoinsText (Variables|/Game/ThirdPerson/Blueprints/BP_ThirdPersonCharacter.BP_ThirdPersonCharacter_C|GetHUD%20Widget (Variables|Default|GetPlayer))) (Utilities|Text|FormatText "Coins: {Coins}" (Variables|Default|GetWallet))))

(fn AddCoins
  (params (Coin :type Integer))
  (bind _output_get (Variables|Default|SetWallet (+ Coin (Variables|Default|GetWallet))))
  (Rendering|Components|TextRender|SetText (Variables|/Game/Dynamic/UI/WB_PlayerStatsHUD.WB_PlayerStatsHUD_C|GetCoinsText (Variables|/Game/ThirdPerson/Blueprints/BP_ThirdPersonCharacter.BP_ThirdPersonCharacter_C|GetHUD%20Widget (Variables|Default|GetPlayer))) (Utilities|Text|FormatText "Coins: {Coins}" _output_get)))