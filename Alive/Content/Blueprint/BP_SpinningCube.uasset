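; BP_SpinningCube is a short-lived Actor that spins erratically around its vertical axis, then removes itself.
; Each Tick adds a large random positive or negative offset to the current yaw, keeping pitch and roll, without scaling by delta time.
; BeginPlay starts a short Delay, after which the actor destroys itself.
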(event EventTick
  (params (DeltaSeconds :type Float%20%28single-precision%29))
  (bind _self self)
  (bind _returnvalue (Transformation|GetActorRotation _self))
  (Transformation|SetActorRotation self (Math|Rotator|MakeRotator (.roll _returnvalue) (.pitch _returnvalue) (+ (.yaw _returnvalue) (Math|Random|RandomFloatinRange -1e+03 1e+03)))))

(event EventBeginPlay
  (Utilities|FlowControl|Delay 3.0)
  (Actor|DestroyActor self))

(fn ConstructionScript)